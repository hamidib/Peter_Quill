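; Player-controlled ship that flies by physics, with input axes for pitch, roll, yaw and engine thrust.
; Each rotation axis drives a pair of thruster components, deactivated at zero input, while engine thrust applies an impulse to the hull along the root arrow's forward vector.
; Tick tints three burner dynamic materials from black to cyan using summed hull velocity components.
; An unconnected check meant to block reverse movement never runs.
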(event `self.ReceiveBeginPlay`
  (bind _returnvalue (`PrimitiveComponent.CreateDynamicMaterialInstance` (`self.EngineRBurner`) 0 "/Game/Materials/MI_EngineThrust.MI_EngineThrust"))
  (set `self.MD_EngineLBurner` _returnvalue)
  (bind _returnvalue_2 (`PrimitiveComponent.CreateDynamicMaterialInstance` (`self.EngineLBurner`) 0 "/Game/Materials/MI_EngineThrust.MI_EngineThrust"))
  (set `self.MD_EngineRBurner` _returnvalue_2)
  (bind _returnvalue_3 (`PrimitiveComponent.CreateDynamicMaterialInstance` (`self.EngineTBurner`) 0 "/Game/Materials/MI_EngineThrust.MI_EngineThrust"))
  (set `self.MD_EngineTBurner` _returnvalue_3))

(event `self.ReceiveTick`
  (params (DeltaSeconds :type "Float (single-precision)"))
  (bind (_returnvalue_x _returnvalue_y _returnvalue_z) (`KismetMathLibrary.BreakVector` (`SceneComponent.GetComponentVelocity` (`self.ShipHull`))))
  (bind _returnvalue (`KismetMathLibrary.LinearColorLerp` (struct :`A` 1.0) (struct :`G` 1.0 :`B` 0.960313 :`A` 1.0) (`KismetMathLibrary.Abs` (/ (+ _returnvalue_x _returnvalue_y _returnvalue_z) 5.0))))
  (`MaterialInstanceDynamic.SetVectorParameterValue` (`self.MD_EngineLBurner`) "Color" _returnvalue)
  (`MaterialInstanceDynamic.SetVectorParameterValue` (`self.MD_EngineRBurner`) "Color" _returnvalue)
  (`MaterialInstanceDynamic.SetVectorParameterValue` (`self.MD_EngineTBurner`) "Color" _returnvalue))

(event `InputAxis|Pitch`
  (params (AxisValue :type "Float (single-precision)"))
  (bind _nosepitchthrust (`self.NosePitchThrust`))
  (bind _tailpitchthrust (`self.TailPitchThrust`))
  ;[1 1 1] Controls Ship Pitch
  (if (!= AxisValue 0.0)
    (bind _output_get (set `PhysicsThrusterComponent.ThrustStrength` (* AxisValue (`self.PitchStrength`)) _nosepitchthrust))
    (set `PhysicsThrusterComponent.ThrustStrength` _output_get _tailpitchthrust)
    (`ActorComponent.Activate` _nosepitchthrust false)
    (`ActorComponent.Activate` _tailpitchthrust false)
    (else
      (`ActorComponent.Deactivate` (`self.NosePitchThrust`))
      (`ActorComponent.Deactivate` (`self.TailPitchThrust`)))))

(event `InputAxis|Roll`
  (params (AxisValue :type "Float (single-precision)"))
  (bind _leftrollthrust (`self.LeftRollThrust`))
  (bind _rightrollthrust (`self.RightRollThrust`))
  ;[1 1 1] Controls Ship Roll
  (if (!= AxisValue 0.0)
    (bind _output_get (set `PhysicsThrusterComponent.ThrustStrength` (* AxisValue (`self.RollStrength`)) _leftrollthrust))
    (set `PhysicsThrusterComponent.ThrustStrength` _output_get _rightrollthrust)
    (`ActorComponent.Activate` _leftrollthrust false)
    (`ActorComponent.Activate` _rightrollthrust false)
    (else
      (`ActorComponent.Deactivate` (`self.LeftRollThrust`))
      (`ActorComponent.Deactivate` (`self.RightRollThrust`)))))

(event `InputAxis|Yaw`
  (params (AxisValue :type "Float (single-precision)"))
  (bind _noseyawthrust (`self.NoseYawThrust`))
  (bind _tailyawthrust (`self.TailYawThrust`))
  ;[1 1 1] Controls Ship Yaw
  (if (!= AxisValue 0.0)
    (bind _output_get (set `PhysicsThrusterComponent.ThrustStrength` (* AxisValue (`self.YawStrength`)) _noseyawthrust))
    (set `PhysicsThrusterComponent.ThrustStrength` _output_get _tailyawthrust)
    (`ActorComponent.Activate` _noseyawthrust false)
    (`ActorComponent.Activate` _tailyawthrust false)
    (else
      (`ActorComponent.Deactivate` (`self.NoseYawThrust`))
      (`ActorComponent.Deactivate` (`self.TailYawThrust`)))))

(event `InputAxis|EngineThrust`
  (params (AxisValue :type "Float (single-precision)"))
  ;[1 1 1] Controls Ships Engine Thrust
  (`PrimitiveComponent.AddImpulse` (`self.ShipHull`) (* (`KismetMathLibrary.GetForwardVector` (`SceneComponent.K2_GetComponentRotation` (`self.RootDirectionArrow`))) (* AxisValue (`self.EnginePower`))) "None" false))

(fn `UserConstructionScript`)