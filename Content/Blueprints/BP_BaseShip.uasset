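; Base player-flyable spaceship with six-degree-of-freedom movement driven by input axes.
; Thrust input eases a persistent desired speed toward forward or half-speed reverse limits, and Tick interpolates current speed toward it to move the hull with sweep.
; Other axes directly rotate or strafe the hull, with vertical sharing the horizontal strength, and mesh hits zero current speed.
; Three dynamic burner materials shift from black to cyan based on summed hull velocity components.
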(event `self.ReceiveBeginPlay`
  (bind _returnvalue (`PrimitiveComponent.CreateDynamicMaterialInstance` (`self.EngineRBurner`) 0 "/Game/Materials/MI_EngineThrust.MI_EngineThrust"))
  (set `self.MD_EngineLBurner` _returnvalue)
  (bind _returnvalue_2 (`PrimitiveComponent.CreateDynamicMaterialInstance` (`self.EngineLBurner`) 0 "/Game/Materials/MI_EngineThrust.MI_EngineThrust"))
  (set `self.MD_EngineRBurner` _returnvalue_2)
  (bind _returnvalue_3 (`PrimitiveComponent.CreateDynamicMaterialInstance` (`self.EngineTBurner`) 0 "/Game/Materials/MI_EngineThrust.MI_EngineThrust"))
  (set `self.MD_EngineTBurner` _returnvalue_3))

(event `self.ReceiveTick`
  (params (DeltaSeconds :type "Float (single-precision)"))
  (bind (_returnvalue_x _returnvalue_y _returnvalue_z) (`KismetMathLibrary.BreakVector` (`SceneComponent.GetComponentVelocity` (`self.ShipHull`))))
  (bind _returnvalue (`KismetMathLibrary.LinearColorLerp` (struct :`A` 1.0) (struct :`G` 1.0 :`B` 0.960313 :`A` 1.0) (`KismetMathLibrary.Abs` (/ (+ _returnvalue_x _returnvalue_y _returnvalue_z) 5.0))))
  ;[1 1 1] Tick - Move Forward/Backward
  (bind _output_get (set `self.CurrentSpeed` (`KismetMathLibrary.FInterpTo` (`self.CurrentSpeed`) (`self.DesiredSpeed`) (`GameplayStatics.GetWorldDeltaSeconds`) (/ (`self.AccelerationInterp`) 2.0))))
  (`SceneComponent.K2_AddLocalOffset` (`self.ShipHull`) (`KismetMathLibrary.MakeVector` _output_get) true false)
  (`MaterialInstanceDynamic.SetVectorParameterValue` (`self.MD_EngineLBurner`) "Color" _returnvalue)
  (`MaterialInstanceDynamic.SetVectorParameterValue` (`self.MD_EngineRBurner`) "Color" _returnvalue)
  (`MaterialInstanceDynamic.SetVectorParameterValue` (`self.MD_EngineTBurner`) "Color" _returnvalue))

(event `InputAxis|EngineThrust`
  (params (AxisValue :type "Float (single-precision)"))
  ;[1 1 1] Forward/Backward Movement
  (if (> AxisValue 0.0)
    (set `self.DesiredSpeed` (`KismetMathLibrary.FInterpTo` (`self.DesiredSpeed`) (`self.MaxSpeed`) (`GameplayStatics.GetWorldDeltaSeconds`) (`self.AccelerationInterp`)))
    (elif (< AxisValue 0.0)
      (set `self.DesiredSpeed` (`KismetMathLibrary.FInterpTo` (`self.DesiredSpeed`) (* (`self.MaxSpeed`) -0.5) (`GameplayStatics.GetWorldDeltaSeconds`) (`self.AccelerationInterp`))))))

(event `InputAxis|Yaw`
  (params (AxisValue :type "Float (single-precision)"))
  ;[1 1 1] Yaw Movement
  (if (!= AxisValue 0.0)
    (`SceneComponent.K2_AddLocalRotation` (`self.ShipHull`) (`KismetMathLibrary.MakeRotator` 0.0 0.0 AxisValue) false false)))

(event `InputAxis|Pitch`
  (params (AxisValue :type "Float (single-precision)"))
  ;[1 1 1] Pitch Movement
  (if (!= AxisValue 0.0)
    (`SceneComponent.K2_AddLocalRotation` (`self.ShipHull`) (`KismetMathLibrary.MakeRotator` 0.0 AxisValue) false false)))

(event `InputAxis|HorizontalMovement`
  (params (AxisValue :type "Float (single-precision)"))
  ;[1 1 1] Controls Horizontal Movement
  (if (!= AxisValue 0.0)
    (`SceneComponent.K2_AddLocalOffset` (`self.ShipHull`) (`KismetMathLibrary.MakeVector` 0.0 (* AxisValue (`self.HorizontalStrength`))) true false)))

(event `InputAxis|VerticalMovement`
  (params (AxisValue :type "Float (single-precision)"))
  ;[1 1 1] Controls Vertical Movement
  (if (!= AxisValue 0.0)
    (`SceneComponent.K2_AddLocalOffset` (`self.ShipHull`) (`KismetMathLibrary.MakeVector` 0.0 0.0 (* AxisValue (`self.HorizontalStrength`))) true false)))

(event `InputAxis|Roll`
  (params (AxisValue :type "Float (single-precision)"))
  ;[1 1 1] Controls Roll Movement
  (if (!= AxisValue 0.0)
    (`SceneComponent.K2_AddLocalRotation` (`self.ShipHull`) (`KismetMathLibrary.MakeRotator` AxisValue) false false)))

(event `self.ShipMesh.OnComponentHit`
  (params (HitComponent :type "PrimitiveComponent Object Reference") (OtherActor :type "Actor Object Reference") (OtherComp :type "PrimitiveComponent Object Reference") (NormalImpulse :type "Vector Structure") (Hit :type "HitResult Structure (by ref)"))
  (set `self.CurrentSpeed` 0.0))

(fn `UserConstructionScript`)