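; Player-controlled base spaceship with six-axis flight, rapid laser fire and engine effects.
; Axis inputs rotate and strafe the hull; thrust eases a desired speed that Tick follows with swept movement and engine glow, while timelines adjust engine pitch.
; Firing loops through a delayed DoOnce to spawn projectiles, and any overlap zeroes current speed.
; BeginPlay creates the HUD widget and burner materials, then tallies UFO enemies by class, though Ai_UFO_Child_blue is left uncounted.
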(event `self.ReceiveActorBeginOverlap`
  (params (OtherActor :type "Actor Object Reference"))
  (set `self.CurrentSpeed` 0.0))

(event `self.ReceiveBeginPlay`
  (`|ExecutionSequence`
    (:`then_0`
      ;[1 1 1] Create players HUD and set dynamic Materials used for Busters
      (bind _returnvalue (`|CreateWidget` "/Game/UI/W_PlayerHUD.W_PlayerHUD_C"))
      (set `self.GameHud` _returnvalue)
      (bind _returnvalue_2 (`PrimitiveComponent.CreateDynamicMaterialInstance` (`self.EngineRBurner`) 0 "/Game/Materials/MI_EngineThrust.MI_EngineThrust"))
      (set `self.MD_EngineLBurner` _returnvalue_2)
      (bind _returnvalue_3 (`PrimitiveComponent.CreateDynamicMaterialInstance` (`self.EngineLBurner`) 0 "/Game/Materials/MI_EngineThrust.MI_EngineThrust"))
      (set `self.MD_EngineRBurner` _returnvalue_3)
      (bind _returnvalue_4 (`PrimitiveComponent.CreateDynamicMaterialInstance` (`self.EngineTBurner`) 0 "/Game/Materials/MI_EngineThrust.MI_EngineThrust"))
      (set `self.MD_EngineTBurner` _returnvalue_4))
    (:`then_1`
      (`self.CalcNumEnemies`))))

(event `self.ReceiveTick`
  (params (DeltaSeconds :type "Float (single-precision)"))
  (bind _returnvalue (`KismetMathLibrary.LinearColorLerp` (struct :`A` 1.0) (struct :`G` 1.0 :`B` 0.960313 :`A` 1.0) (`KismetMathLibrary.Abs` (/ (`self.CurrentSpeed`) 2.0))))
  ;[1 1 1] Tick - Move Forward/Backward
  (bind _output_get (set `self.CurrentSpeed` (`KismetMathLibrary.FInterpTo` (`self.CurrentSpeed`) (`self.DesiredSpeed`) (`GameplayStatics.GetWorldDeltaSeconds`) (/ (`self.AccelerationInterp`) 2.0))))
  (`SceneComponent.K2_AddLocalOffset` (`self.ShipHull`) (`KismetMathLibrary.MakeVector` _output_get) true false)
  ;[1 1 1] Shade Engine busters
  (`MaterialInstanceDynamic.SetVectorParameterValue` (`self.MD_EngineLBurner`) "Color" _returnvalue)
  (`MaterialInstanceDynamic.SetVectorParameterValue` (`self.MD_EngineRBurner`) "Color" _returnvalue)
  (`MaterialInstanceDynamic.SetVectorParameterValue` (`self.MD_EngineTBurner`) "Color" _returnvalue))

(event `InputAxis|EngineThrust`
  (params (AxisValue :type "Float (single-precision)"))
  ;[1 1 1] Forward/Backward Movement
  (if (> AxisValue 0.0)
    (bind (_direction _engine_pitch) (`Timeline|engine pitch`)
      (:`Update`
        (`AudioComponent.SetPitchMultiplier` (`self.engine`) _engine_pitch)
        (set `self.DesiredSpeed` (`KismetMathLibrary.FInterpTo` (`self.DesiredSpeed`) (`self.MaxSpeed`) (`GameplayStatics.GetWorldDeltaSeconds`) (`self.AccelerationInterp`)))))
    (else
      (bind (_direction_2 _engine_pitch_2) (`Timeline|Timeline_0` :!via `Reverse`)
        (:`Update`
          (`AudioComponent.SetPitchMultiplier` (`self.engine`) _engine_pitch_2)
          (if (< AxisValue 0.0)
            (set `self.DesiredSpeed` (`KismetMathLibrary.FInterpTo` (`self.DesiredSpeed`) (* (`self.MaxSpeed`) -0.5) (`GameplayStatics.GetWorldDeltaSeconds`) (`self.AccelerationInterp`)))))))))

(event `InputAxis|Yaw`
  (params (AxisValue :type "Float (single-precision)"))
  ;[1 1 1] Yaw Movement
  (if (!= AxisValue 0.0)
    (`SceneComponent.K2_AddLocalRotation` (`self.ShipHull`) (`KismetMathLibrary.MakeRotator` 0.0 0.0 AxisValue) false false)))

(event `InputAxis|Pitch`
  (params (AxisValue :type "Float (single-precision)"))
  ;[1 1 1] Pitch Movement
  (if (!= AxisValue 0.0)
    (`SceneComponent.K2_AddLocalRotation` (`self.ShipHull`) (`KismetMathLibrary.MakeRotator` 0.0 AxisValue) false false)))

(event `InputAxis|HorizontalMovement`
  (params (AxisValue :type "Float (single-precision)"))
  ;[1 1 1] Controls Horizontal Movement
  (if (!= AxisValue 0.0)
    (`SceneComponent.K2_AddLocalOffset` (`self.ShipHull`) (`KismetMathLibrary.MakeVector` 0.0 (* AxisValue (`self.HorizontalStrength`))) true false)))

(event `InputAxis|VerticalMovement`
  (params (AxisValue :type "Float (single-precision)"))
  ;[1 1 1] Controls Vertical Movement
  (if (!= AxisValue 0.0)
    (`SceneComponent.K2_AddLocalOffset` (`self.ShipHull`) (`KismetMathLibrary.MakeVector` 0.0 0.0 (* AxisValue (`self.HorizontalStrength`))) true false)))

(event `InputAxis|Roll`
  (params (AxisValue :type "Float (single-precision)"))
  ;[1 1 1] Controls Roll Movement
  (if (!= AxisValue 0.0)
    (`SceneComponent.K2_AddLocalRotation` (`self.ShipHull`) (`KismetMathLibrary.MakeRotator` AxisValue) false false)))

(event `InputAction|FireWeapons`
  (params (Key :type "Key Structure"))
  ;[1 1 1] Controls Firing State
  (:`Pressed`
    (`self.Firing` true))
  (:`Released`
    (`self.Firing` false)))

(event `Firing`
  (params (FiringWeapons :type Boolean))
  ;[1 1 1] Performs Rapid Fire
  (set `self.FiringWeapons` FiringWeapons)
  (if (`self.FiringWeapons`) :!label _label
    (`/Engine/EditorBlueprintResources/StandardMacros.DoOnce` false :!label _label_2
      (:`Completed`
        (`self.FireWeapons`)
        (`KismetSystemLibrary.Delay` 0.1)
        (`|ExecutionSequence`
          (:`then_0`
            (goto _label_2 :!via `Reset`))
          (:`then_1`
            (goto _label)))))))

(fn `CalcNumEnemies`
  (`|ExecutionSequence`
    (:`then_0`
      (bind _outactors (`GameplayStatics.GetAllActorsOfClass` "/Game/Imports/FlyingBP/Blueprints/ai_UFO_blue.ai_UFO_blue_C"))
      (`KismetSystemLibrary.PrintString` "Number of ai_UFO_blue is: ")
      (bind _returnvalue (`KismetArrayLibrary.Array_Length` _outactors))
      (`KismetSystemLibrary.PrintString` (`KismetStringLibrary.Conv_IntToString` _returnvalue))
      (set `self.NumberOfEnemies` (+ _returnvalue (`self.NumberOfEnemies`))))
    (:`then_1`
      (bind _outactors_2 (`GameplayStatics.GetAllActorsOfClass` "/Game/Imports/FlyingBP/Blueprints/ai_UFO_Boss_blue.ai_UFO_Boss_blue_C"))
      (`KismetSystemLibrary.PrintString` "Number of ai_UFO_Boss_blue is: ")
      (bind _returnvalue_2 (`KismetArrayLibrary.Array_Length` _outactors_2))
      (`KismetSystemLibrary.PrintString` (`KismetStringLibrary.Conv_IntToString` _returnvalue_2))
      (set `self.NumberOfEnemies` (+ _returnvalue_2 (`self.NumberOfEnemies`))))
    (:`then_2`
      (bind _outactors_3 (`GameplayStatics.GetAllActorsOfClass` "/Game/Imports/FlyingBP/Blueprints/ai_UFO_Boss_blue_Mini.ai_UFO_Boss_blue_Mini_C"))
      (`KismetSystemLibrary.PrintString` "Number of ai_UFO_Boss_blue_mini is: ")
      (bind _returnvalue_3 (`KismetArrayLibrary.Array_Length` _outactors_3))
      (`KismetSystemLibrary.PrintString` (`KismetStringLibrary.Conv_IntToString` _returnvalue_3))
      (set `self.NumberOfEnemies` (+ _returnvalue_3 (`self.NumberOfEnemies`))))
    (:`then_3`
      (bind _outactors_4 (`GameplayStatics.GetAllActorsOfClass` "/Game/Imports/FlyingBP/Blueprints/ai_UFO_Boss_blue_Mini1.ai_UFO_Boss_blue_Mini1_C"))
      (`KismetSystemLibrary.PrintString` "Number of ai_UFO_Boss_blue_mini_1 is: ")
      (bind _returnvalue_4 (`KismetArrayLibrary.Array_Length` _outactors_4))
      (`KismetSystemLibrary.PrintString` (`KismetStringLibrary.Conv_IntToString` _returnvalue_4))
      (set `self.NumberOfEnemies` (+ _returnvalue_4 (`self.NumberOfEnemies`))))
    (:`then_4`
      (bind _outactors_5 (`GameplayStatics.GetAllActorsOfClass` "/Game/Imports/FlyingBP/Blueprints/ai_UFO_Boss_Child+Blue.ai_UFO_Boss_Child+Blue_C"))
      (`KismetSystemLibrary.PrintString` "Number of ai_UFO_Boss_Child+Blueis: ")
      (bind _returnvalue_5 (`KismetArrayLibrary.Array_Length` _outactors_5))
      (`KismetSystemLibrary.PrintString` (`KismetStringLibrary.Conv_IntToString` _returnvalue_5))
      (set `self.NumberOfEnemies` (+ _returnvalue_5 (`self.NumberOfEnemies`))))
    (:`then_5`
      (bind _outactors_6 (`GameplayStatics.GetAllActorsOfClass` "/Game/Imports/FlyingBP/Blueprints/ai_UFO_Boss_Child_Blue.ai_UFO_Boss_Child_Blue_C"))
      (`KismetSystemLibrary.PrintString` "Number of ai_UFO_Boss_Child_blue is: ")
      (bind _returnvalue_6 (`KismetArrayLibrary.Array_Length` _outactors_6))
      (`KismetSystemLibrary.PrintString` (`KismetStringLibrary.Conv_IntToString` _returnvalue_6))
      (set `self.NumberOfEnemies` (+ _returnvalue_6 (`self.NumberOfEnemies`))))
    (:`then_6`
      (bind _outactors_7 (`GameplayStatics.GetAllActorsOfClass` "/Game/Imports/FlyingBP/Blueprints/ai_UFO_Boss_Child_Green.ai_UFO_Boss_Child_Green_C"))
      (`KismetSystemLibrary.PrintString` "Number of ai_UFO_Boss_Child_green is: ")
      (bind _returnvalue_7 (`KismetArrayLibrary.Array_Length` _outactors_7))
      (`KismetSystemLibrary.PrintString` (`KismetStringLibrary.Conv_IntToString` _returnvalue_7))
      (set `self.NumberOfEnemies` (+ _returnvalue_7 (`self.NumberOfEnemies`))))
    (:`then_7`
      (bind _outactors_8 (`GameplayStatics.GetAllActorsOfClass` "/Game/Imports/FlyingBP/Blueprints/ai_UFO_Boss_green_Mini.ai_UFO_Boss_green_Mini_C"))
      (`KismetSystemLibrary.PrintString` "Number of ai_UFO_Boss_green_mini is: ")
      (bind _returnvalue_8 (`KismetArrayLibrary.Array_Length` _outactors_8))
      (`KismetSystemLibrary.PrintString` (`KismetStringLibrary.Conv_IntToString` _returnvalue_8))
      (set `self.NumberOfEnemies` (+ _returnvalue_8 (`self.NumberOfEnemies`))))
    (:`then_8`
      (bind _outactors_9 (`GameplayStatics.GetAllActorsOfClass` "/Game/Imports/FlyingBP/Blueprints/ai_UFO_Child_blue.ai_UFO_Child_blue_C"))
      (`KismetSystemLibrary.PrintString` "Number of ai_UFO_Child_blue is: ")
      (`KismetSystemLibrary.PrintString` (`KismetStringLibrary.Conv_IntToString` (`KismetArrayLibrary.Array_Length` _outactors_9))))
    (:`then_9`
      (bind _outactors_10 (`GameplayStatics.GetAllActorsOfClass` "/Game/Imports/FlyingBP/Blueprints/ai_UFO_Child_Green.ai_UFO_Child_Green_C"))
      (`KismetSystemLibrary.PrintString` "Number of ai_UFO_Child_Green is: ")
      (bind _returnvalue_9 (`KismetArrayLibrary.Array_Length` _outactors_10))
      (`KismetSystemLibrary.PrintString` (`KismetStringLibrary.Conv_IntToString` _returnvalue_9))
      (set `self.NumberOfEnemies` (+ _returnvalue_9 (`self.NumberOfEnemies`))))
    (:`then_10`
      (bind _outactors_11 (`GameplayStatics.GetAllActorsOfClass` "/Game/Imports/FlyingBP/Blueprints/ai_UFO_Parent.ai_UFO_Parent_C"))
      (`KismetSystemLibrary.PrintString` "Number of ai_UFO_Parent is: ")
      (bind _returnvalue_10 (`KismetArrayLibrary.Array_Length` _outactors_11))
      (`KismetSystemLibrary.PrintString` (`KismetStringLibrary.Conv_IntToString` _returnvalue_10))
      (set `self.NumberOfEnemies` (+ _returnvalue_10 (`self.NumberOfEnemies`))))
    (:`then_11`
      (bind _outactors_12 (`GameplayStatics.GetAllActorsOfClass` "/Game/Imports/FlyingBP/Blueprints/ai_UFO_Parent_Boss.ai_UFO_Parent_Boss_C"))
      (`KismetSystemLibrary.PrintString` "Number of ai_UFO_Parent_Boss is: ")
      (bind _returnvalue_11 (`KismetArrayLibrary.Array_Length` _outactors_12))
      (`KismetSystemLibrary.PrintString` (`KismetStringLibrary.Conv_IntToString` _returnvalue_11))
      (set `self.NumberOfEnemies` (+ _returnvalue_11 (`self.NumberOfEnemies`)))
      (`KismetSystemLibrary.PrintString` "Total Ships is: ")
      (`KismetSystemLibrary.PrintString` (`KismetStringLibrary.Conv_IntToString` (`self.NumberOfEnemies`))))))

(fn `FireWeapons`
  (bind _returnvalue (`SceneComponent.K2_GetComponentRotation` (`self.ShipHull`)))
  (`|SpawnActorFromClass` "/Game/Blueprints/Weapons/Projectiles/LaserProjectile.LaserProjectile_C" (`KismetMathLibrary.MakeTransform` (+ (`SceneComponent.K2_GetComponentLocation` (`self.ShipHull`)) (`KismetMathLibrary.GreaterGreater_VectorRotator` (`self.Gunoffset`) _returnvalue)) _returnvalue) "Undefined" "OverrideRootScale" null null)
  (`GameplayStatics.PlaySoundAtLocation` "/Engine/VREditor/Sounds/UI/Laser_Pull.Laser_Pull" (`self.K2_GetActorLocation`)))

(fn `UserConstructionScript`)